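; Base tic-tac-toe piece pawn for X and O, picked up by click or touch and placed on grid boxes.
; Carrying spring-interpolates toward the mouse ray's Z=0 intersection, while overlapping Grid_Selectable boxes validate moves.
; Placing springs it to the box center, writes TTTGameMode's grid, spawns a replacement at the original transform and updates TicTacToeController's possession.
; It then increments the move count and prints the win check result.
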(event MouseInput|EventActorBeginCursorOver
  ;[1 1 1] handle selection and deselection of pawn
  (Variables|CarryingPawn|SetisHovering true))

(event Collision|EventActorBeginOverlap
  (params (OtherActor :type Actor%20Object%20Reference))
  (bind _overlappedbox (Variables|MakingAMove|GetoverlappedBox))
  (bind _returnvalue (Utilities|Array|LastIndex _overlappedbox))
  ;[1 1 1] Hover over pieces and check if a valid move
  (if (== (Utilities|GetClass OtherActor) "/Game/Blueprints/Grid_Selectable.Grid_Selectable_C")
    (Utilities|Array|SetArrayElem _overlappedbox (+ _returnvalue 1) OtherActor true)
    (bind _asgrid_selectable (Utilities|Casting|CastToGrid_Selectable (Utilities|Array|Get(acopy) _overlappedbox _returnvalue)))
    (bind _iscompatible (Default|CheckCompat _asgrid_selectable))
    (Variables|MakingaMove|SetisMoveAllowed _iscompatible)))

(event EventTick
  (params (DeltaSeconds :type Float%20%28single-precision%29))
  (if (Variables|CarryingPawn|GetshouldCarryWithMouse)
    ;[1 1 1] Carry Pawn With mouse
    (CallFunction|CarryPawn)
    (else
      ;[1 1 1] Post move lerping to grid box center
      (if (Math|Vector|NotEqual(Vector) (Variables|MakingAMove|GetfinalLerpToLocation) "0, 0, 0" 0.0001)
        (CallFunction|AutoLerptoLoc)))))

(event Collision|EventActorEndOverlap
  (params (OtherActor :type Actor%20Object%20Reference))
  ;[1 1 1] Hover over pieces and check if a valid move
  (if (== "/Game/Blueprints/Grid_Selectable.Grid_Selectable_C" (Utilities|GetClass OtherActor))
    (Utilities|Array|RemoveItem (Variables|MakingAMove|GetoverlappedBox) OtherActor)))

(event MouseInput|EventActorEndCursorOver
  ;[1 1 1] handle selection and deselection of pawn
  (Variables|CarryingPawn|SetisHovering false))

(event EventBeginPlay
  (bind _returnvalue (Game|GetPlayerController 0))
  (bind _self self)
  (bind _myvalue (Variables|MakingaMove|GetmyValue))
  ;[1 1 1] Start()
  (Input|EnableInput _returnvalue)
  (Variables|MakingaMove|SetmySpawnTransform (Transformation|GetWorldTransform (Variables|Default|GetScene)))
  (bind _astic_tac_toe_controller (Utilities|Casting|CastToTicTacToeController _returnvalue))
  (Default|TogglePossessed _astic_tac_toe_controller)
  (Default|ChoosePossessed _astic_tac_toe_controller _myvalue self)
  (if (== _myvalue -1)
    (Variables|/Game/Blueprints/Game/TicTacToeController.TicTacToeController_C|SetnewestX _astic_tac_toe_controller _self)
    (else
      (Variables|/Game/Blueprints/Game/TicTacToeController.TicTacToeController_C|SetnewestO _astic_tac_toe_controller _self))))

(event Input|MouseEvents|LeftMouseButton
  (params (Key :type Key%20Structure :default "None"))
  (bind _overlappedbox (Variables|MakingAMove|GetoverlappedBox))
  ;[1 1 1] handle selection and deselection of pawn
  (:Pressed
    (if (Variables|MakingaMove|GetisMoveAllowed)
      (bind _asgrid_selectable (Utilities|Casting|CastToGrid_Selectable (Utilities|Array|Get(acopy) _overlappedbox (Utilities|Array|LastIndex _overlappedbox))))
      (Variables|MakingAMove|SetfinalLerpToLocation (Transformation|GetActorLocation _asgrid_selectable))
      (Variables|MakingaMove|SetmoveGridIndex (Variables|/Game/Blueprints/Grid_Selectable.Grid_Selectable_C|GetmyIndex _asgrid_selectable))
      (CallFunction|MakeMove)
      (elif (Variables|CarryingPawn|GetisHovering)
        (Variables|CarryingPawn|SetshouldCarryWithMouse (not (Variables|CarryingPawn|GetshouldCarryWithMouse)))))))

(event Input|TouchEvents|Touch1
  (params (Key :type Key%20Structure :default "None"))
  (bind _overlappedbox (Variables|MakingAMove|GetoverlappedBox))
  ;[1 1 1] handle selection and deselection of pawn
  (:Pressed
    (if (Variables|MakingaMove|GetisMoveAllowed)
      (bind _asgrid_selectable (Utilities|Casting|CastToGrid_Selectable (Utilities|Array|Get(acopy) _overlappedbox (Utilities|Array|LastIndex _overlappedbox))))
      (Variables|MakingAMove|SetfinalLerpToLocation (Transformation|GetActorLocation _asgrid_selectable))
      (Variables|MakingaMove|SetmoveGridIndex (Variables|/Game/Blueprints/Grid_Selectable.Grid_Selectable_C|GetmyIndex _asgrid_selectable))
      (CallFunction|MakeMove)
      (elif (Variables|CarryingPawn|GetisHovering)
        (Variables|CarryingPawn|SetshouldCarryWithMouse (not (Variables|CarryingPawn|GetshouldCarryWithMouse)))))))

(fn ConstructionScript)

(fn MakeMove
  (bind _myvalue (Variables|MakingaMove|GetmyValue))
  (bind _astttgame_mode (Utilities|Casting|CastToTTTGameMode (Game|GetGameMode)))
  (Utilities|FlowControl|Sequence
    (:then_0
      ;[1 1 1] set grid index
      (if (> (Variables|MakingaMove|GetmoveGridIndex) -1)
        (Development|PrintString (Utilities|String|ToString(Integer) (Variables|MakingaMove|GetmoveGridIndex)))
        (Utilities|Array|SetArrayElem (Variables|/Game/Blueprints/Game/TTTGameMode.TTTGameMode_C|GetGridInfo _astttgame_mode) (Variables|MakingaMove|GetmoveGridIndex) (Variables|MakingaMove|GetmyValue) true)
        (else
          (return))))
    (:then_1
      ;[1 1 1] lerp to selection center
      (Variables|MakingaMove|SetshouldPostMoveLerp true)
      (Variables|CarryingPawn|SetisHovering false)
      (Variables|CarryingPawn|SetshouldCarryWithMouse false))
    (:then_2
      ;[1 1 1] spawn new at original place, and tell controller about it
      (bind _returnvalue (Game|SpawnActorfromClass (Utilities|GetClass self) (Variables|MakingaMove|GetmySpawnTransform) "Undefined" 0 0))
      (bind _astic_tac_toe_controller (Utilities|Casting|CastToTicTacToeController (Game|GetPlayerController 0)))
      (if (== _myvalue -1)
        (Variables|/Game/Blueprints/Game/TicTacToeController.TicTacToeController_C|SetnewestX _astic_tac_toe_controller _returnvalue)
        (else
          (Variables|/Game/Blueprints/Game/TicTacToeController.TicTacToeController_C|SetnewestO _astic_tac_toe_controller _returnvalue))))
    (:then_3
      ;[1 1 1] call set new possession on controller, where it has refs to latest copies of x and zero
      (Default|SetPostMovePossession _astic_tac_toe_controller _myvalue)
      (Variables|MakingaMove|SetisMoveAllowed false))
    (:then_4
      ;[1 1 1] determine whether game is over or no
      (bind _astttgame_mode_2 (Utilities|Casting|CastToTTTGameMode (Game|GetGameMode)))
      (Default|IncreaseMoveCount _astttgame_mode_2)
      (bind _result (Default|DidThisMoveWin _astttgame_mode_2 (Variables|MakingaMove|GetmoveGridIndex)))
      (Variables|MakingaMove|SetmoveGridIndex -1)
      (Development|PrintString (Utilities|String|ToString(Boolean) _result)))))

(fn CarryPawn
  (bind _returnvalue (Game|GetPlayerController 0))
  (bind _scene (Variables|Default|GetScene))
  (bind (_worldlocation _worlddirection) (Game|Player|ConvertMouseLocationToWorldSpace _returnvalue))
  (bind _output_get (Variables|CarryingPawn|SetcurrentLerpToLocation (+ _worldlocation (* (* _worlddirection (/ (.Z (Math|Vector|BreakVector _worldlocation)) (.Z (Math|Vector|BreakVector _worlddirection)))) -1))))
  (bind _returnvalue_2 (Class|KismetMathLibrary|VectorSpringInterp (Transformation|GetWorldLocation _scene) _output_get (Variables|CarryingPawn|GetSpring%20State) 0.75 0.75 0.1 1.0))
  (Transformation|SetWorldLocation _scene _returnvalue_2 false false))

(fn AutoLerptoLoc
  (bind _scene (Variables|Default|GetScene))
  (bind _returnvalue (Class|KismetMathLibrary|VectorSpringInterp (Transformation|GetWorldLocation _scene) (Variables|MakingAMove|GetfinalLerpToLocation) (Variables|CarryingPawn|GetSpring%20State) 0.75 0.75 0.1 1.0))
  (Transformation|SetWorldLocation _scene _returnvalue false false))