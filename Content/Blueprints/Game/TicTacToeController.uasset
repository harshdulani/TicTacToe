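; Tic-tac-toe controller that switches possession between X and O pawns.
; Shortly after BeginPlay it possesses the newest X pawn, and SetPostMovePossession picks the newest O or X pawn from the value passed in.
; ChoosePossessed lets a candidate pawn take control when its value matches Possessed, or is -1 while Possessed is still zero.
; TogglePossessed flips the side by negating that signed value.
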(event EventBeginPlay
  (Utilities|FlowControl|Delay 0.25)
  (CallFunction|SetPostMovePossession 1))

(fn ConstructionScript)

(fn ChoosePossessed
  (params (candidateValue :type Integer) (pawnReference :type Pawn%20Base%20Object%20Reference))
  ;[1 1 1] Since it's going to be called by both the pawns, the need for checking their values, and if required their refs
  (if (== candidateValue (Variables|Default|Getpossessed))
    (Pawn|Possess pawnReference :!label _label)
    (Variables|Default|Setpossessed candidateValue)
    (elif (and (== (Variables|Default|Getpossessed) 0) (== candidateValue -1))
      (goto _label))))

(fn TogglePossessed
  ;[1 1 1] Toggle desired Possessed between X & 0
  (bind _output_get (Variables|Default|Setpossessed (* (Variables|Default|Getpossessed) -1)))
  (return _output_get))

(fn SetPostMovePossession
  (params (oldValue :type Integer))
  (if (== oldValue -1)
    (bind _aspawn (Utilities|Casting|CastToPawn (Variables|Default|GetnewestO)))
    (Pawn|Possess _aspawn)
    (else
      (bind _aspawn_2 (Utilities|Casting|CastToPawn (Variables|Default|GetnewestX)))
      (Pawn|Possess _aspawn_2))))