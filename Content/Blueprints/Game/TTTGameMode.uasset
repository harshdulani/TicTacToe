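; Tic-tac-toe game mode that counts moves and decides whether a given move wins on the 3x3 GridInfo board.
; DidThisMoveWin returns false under three moves, then checks the move's row and column via modulo math, plus both diagonals for even indices.
; Lines are compared by cell sign using chained XORs, in which the middle cell cancels out, so only the two end cells affect each result.
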(fn ConstructionScript)

(fn DidThisMoveWin
  (params (moveIndex :type Integer))
  (bind _returnvalue (Math|Integer|%(Integer) moveIndex 3))
  (bind _returnvalue_2 (- moveIndex _returnvalue))
  (bind _astttgame_mode (Utilities|Casting|CastToTTTGameMode (Game|GetGameMode)))
  (Utilities|FlowControl|Sequence
    (:then_0
      ;[1 1 1] Cannot win if atleast 3 moves are not made
      (if (< (Variables|Default|GettotalMovesMade) 3)
        (return false)))
    (:then_1
      ;[1 1 1] test patterns in %3 prove horizontal rows
      (if (not (Class|KismetMathLibrary|XORBoolean (Class|KismetMathLibrary|XORBoolean (< (Utilities|Array|Get(acopy) (Variables|TTTGameMode_C|GetGridInfo _astttgame_mode) _returnvalue_2) 0) (< (Utilities|Array|Get(acopy) (Variables|TTTGameMode_C|GetGridInfo _astttgame_mode) (+ _returnvalue_2 1)) 0)) (Class|KismetMathLibrary|XORBoolean (< (Utilities|Array|Get(acopy) (Variables|TTTGameMode_C|GetGridInfo _astttgame_mode) (+ _returnvalue_2 1)) 0) (< (Utilities|Array|Get(acopy) (Variables|TTTGameMode_C|GetGridInfo _astttgame_mode) (+ _returnvalue_2 2)) 0))))
        (return true)))
    (:then_2
      ;[1 1 1] x = i%3. arr[x], arr[x + 3], arr[x + 6] should have same values for column win case check
      (if (not (Class|KismetMathLibrary|XORBoolean (Class|KismetMathLibrary|XORBoolean (< (Utilities|Array|Get(acopy) (Variables|TTTGameMode_C|GetGridInfo _astttgame_mode) _returnvalue) 0) (< (Utilities|Array|Get(acopy) (Variables|TTTGameMode_C|GetGridInfo _astttgame_mode) (+ _returnvalue 3)) 0)) (Class|KismetMathLibrary|XORBoolean (< (Utilities|Array|Get(acopy) (Variables|TTTGameMode_C|GetGridInfo _astttgame_mode) (+ _returnvalue 3)) 0) (< (Utilities|Array|Get(acopy) (Variables|TTTGameMode_C|GetGridInfo _astttgame_mode) (+ _returnvalue 6)) 0))))
        (return true)))
    (:then_3
      ;[1 1 1] all indices that require diagonal checks lie on even nos.
      (if (== (Math|Integer|%(Integer) moveIndex 2) 0)
        (return (or (not (Class|KismetMathLibrary|XORBoolean (Class|KismetMathLibrary|XORBoolean (< (Utilities|Array|Get(acopy) (Variables|TTTGameMode_C|GetGridInfo _astttgame_mode)) 0) (< (Utilities|Array|Get(acopy) (Variables|TTTGameMode_C|GetGridInfo _astttgame_mode) 4) 0)) (Class|KismetMathLibrary|XORBoolean (< (Utilities|Array|Get(acopy) (Variables|TTTGameMode_C|GetGridInfo _astttgame_mode) 4) 0) (< (Utilities|Array|Get(acopy) (Variables|TTTGameMode_C|GetGridInfo _astttgame_mode) 8) 0)))) (not (Class|KismetMathLibrary|XORBoolean (Class|KismetMathLibrary|XORBoolean (< (Utilities|Array|Get(acopy) (Variables|TTTGameMode_C|GetGridInfo _astttgame_mode) 2) 0) (< (Utilities|Array|Get(acopy) (Variables|TTTGameMode_C|GetGridInfo _astttgame_mode) 4) 0)) (Class|KismetMathLibrary|XORBoolean (< (Utilities|Array|Get(acopy) (Variables|TTTGameMode_C|GetGridInfo _astttgame_mode) 4) 0) (< (Utilities|Array|Get(acopy) (Variables|TTTGameMode_C|GetGridInfo _astttgame_mode) 6) 0))))))))
    (:then_4
      (return false))))

(fn IncreaseMoveCount
  (Variables|Default|SettotalMovesMade (+ (Variables|Default|GettotalMovesMade) 1))
  (return))